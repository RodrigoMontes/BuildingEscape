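; Openable door actor that swings open and closed in response to the OnOpen and OnClose events of its OpenDoor component.
; A timeline plays forward or in reverse, and its DoorAngle track sets the yaw, combined with the rotation cached at BeginPlay.
; An event track on the timeline plays the Doorlock sound at the actor's location.
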(event `self.ReceiveBeginPlay`
  (set `self.Initial_Rotation` (`self.K2_GetActorRotation`)))

(event `self.OpenDoor.OnOpen`
  (bind (_direction _door_angle) (`Timeline|Timeline_0` :!label _label)
    (:`Update`
      (`self.K2_SetActorRotation` (`KismetMathLibrary.ComposeRotators` (`KismetMathLibrary.MakeRotator` 0.0 0.0 _door_angle) (`self.Initial_Rotation`))))
    (:`Open Door Sound Cue`
      (`GameplayStatics.PlaySoundAtLocation` "/Game/Audio/door-lock.door-lock" (`self.K2_GetActorLocation`) (struct) 1.0 1.0 0.0 null null null))))

(event `self.OpenDoor.OnClose`
  (goto _label :!via `Reverse`))

(fn `UserConstructionScript`)